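; Melee enemy that chases and punches the player, outlined through custom depth when holding a key.
; Pawn sensing, overlap or taking damage triggers AI MoveTo, then a punch montage whose hand overlaps damage non-dashing players.
; Hits grant optional brief invincibility and play a freezing hurt montage chosen by the player's BigHit flag.
; Death ragdolls it away from the player, changes player blood, clears lock-on and increments its spawner's dead count.
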(event `self.ReceiveBeginPlay`
  (bind _mesh (`self.Mesh`))
  (if (`self.isHoldingKey`)
    (`PrimitiveComponent.SetRenderCustomDepth` _mesh true)
    (`PrimitiveComponent.SetCustomDepthStencilValue` _mesh 1)))

(event `self.ReceiveTick`
  (params (DeltaSeconds :type "Float (single-precision)"))
  ;[1 1 1] Event Tick
  (`|ExecutionSequence`
    (:`then_0`
      (`self.UpdateHealthBar`))
    (:`then_1`
      (if (`self.invincible`)
        (`KismetSystemLibrary.Delay` 0.4)
        (set `self.invincible` false)))
    (:`then_2`
      (if (`self.IsOverlappingActor` (`GameplayStatics.GetPlayerPawn` 0))
        (`self.FollowPlayer`)))))

(event `self.PawnSensing.OnSeePawn`
  (params (Pawn :type "Pawn Object Reference"))
  (`self.FollowPlayer`))

(event `FollowPlayer`
  ;[1 1 1] Chasing Player
  (if (not (`self.frozen`))
    (`|AIMoveTo` self (0.0 0.0 0.0) (`GameplayStatics.GetPlayerCharacter` 0) 70.0
      (:`OnSuccess`
        (if (not (`self.isAttacking`))
          (set `self.isAttacking` true)
          (bind _returnvalue (`self.PlayAnimMontage` "/Game/Characters/Enemy/EnemyPunches_Montage.EnemyPunches_Montage" 2.0))
          (`KismetSystemLibrary.Delay` _returnvalue)
          (set `self.isAttacking` false))))))

(event `self.RightHand.OnComponentBeginOverlap`
  (params (OverlappedComponent :type "PrimitiveComponent Object Reference") (OtherActor :type "Actor Object Reference") (OtherComp :type "PrimitiveComponent Object Reference") (OtherBodyIndex :type Integer) (bFromSweep :type Boolean) (SweepResult :type "HitResult Structure (by ref)"))
  ;[1 1 1] Attack Collision Detection
  (bind _asbp_third_person_character (cast `/Game/Blueprints/BP_ThirdPersonCharacter` OtherActor))
  (if (and (not (`self.frozen`)) (`self.isAttacking`) (not (`/Game/Blueprints/BP_ThirdPersonCharacter.Dashing` _asbp_third_person_character)))
    (`/Game/Blueprints/BP_ThirdPersonCharacter.ChangeHealth` _asbp_third_person_character -2.0)))

(event `self.LeftHand.OnComponentBeginOverlap`
  (params (OverlappedComponent :type "PrimitiveComponent Object Reference") (OtherActor :type "Actor Object Reference") (OtherComp :type "PrimitiveComponent Object Reference") (OtherBodyIndex :type Integer) (bFromSweep :type Boolean) (SweepResult :type "HitResult Structure (by ref)"))
  ;[1 1 1] Attack Collision Detection
  (bind _asbp_third_person_character (cast `/Game/Blueprints/BP_ThirdPersonCharacter` OtherActor))
  (if (and (not (`self.frozen`)) (`self.isAttacking`) (not (`/Game/Blueprints/BP_ThirdPersonCharacter.Dashing` _asbp_third_person_character)))
    (`/Game/Blueprints/BP_ThirdPersonCharacter.ChangeHealth` _asbp_third_person_character -2.0)))

(event `TakeDamage`
  (params (TriggerInvincibility :type Boolean :default true) (Damage :type "Float (double-precision)" :default 50.0) (BloodOffset :type "Float (double-precision)" :default 10.0))
  (bind _mesh (`self.Mesh`))
  (bind _healthbar_w (`self.HealthBar_W`))
  (bind _enemyspawner (`self.EnemySpawner`))
  ;[1 1 1] Take Damange and Die
  (if (not (`self.invincible`))
    (bind _output_get (set `self.Health` (- (`self.Health`) Damage)))
    (set `self.Dead` (<= _output_get 0.0))
    (set `self.invincible` TriggerInvincibility)
    (`GameplayStatics.PlaySound2D` "/Game/Audio/swordHit.swordHit" 1.0 1.0 0.0 null null)
    (if (`self.Dead`)
      (if (`KismetSystemLibrary.IsValid` _healthbar_w)
        (`ActorComponent.K2_DestroyComponent` _healthbar_w)
        (bind _asbp_third_person_character (cast `/Game/Blueprints/BP_ThirdPersonCharacter` (`GameplayStatics.GetPlayerPawn` 0)))
        (`/Game/Blueprints/BP_ThirdPersonCharacter.ChangeBlood` _asbp_third_person_character BloodOffset)
        (set `self.frozen` true)
        (`PrimitiveComponent.SetCollisionEnabled` (`self.CapsuleComponent`) "NoCollision")
        (`PrimitiveComponent.SetSimulatePhysics` _mesh true)
        (`PrimitiveComponent.AddImpulse` _mesh (* (`KismetMathLibrary.GetDirectionUnitVector` (`self.K2_GetActorLocation` (`GameplayStatics.GetPlayerPawn` 0)) (`self.K2_GetActorLocation`)) 20000.0) "None" false)
        (`GameplayStatics.PlaySound2D` "/Game/Audio/died.died" 0.25 1.0 0.0 null null)
        (`self.ClearLockOn`)
        (`/Engine/EditorBlueprintResources/StandardMacros.IsValid` _enemyspawner
          (:`Is Valid`
            (set `/Game/Blueprints/BP_Enemy_Spawner.NumberofDeadEnemies` (+ 1 (`/Game/Blueprints/BP_Enemy_Spawner.NumberofDeadEnemies` _enemyspawner)) _enemyspawner))))
      (else
        (`self.PlayHurt`)
        (`self.FollowPlayer`)))))

(fn `ClearLockOn`
  (bind _asbp_third_person_character (cast `/Game/Blueprints/BP_ThirdPersonCharacter` (`GameplayStatics.GetPlayerPawn` 0)))
  (if (== (`/Game/Blueprints/BP_ThirdPersonCharacter.LockOnTarget` _asbp_third_person_character) self)
    (set `/Game/Blueprints/BP_ThirdPersonCharacter.LockOnTarget` null _asbp_third_person_character)
    (`PrimitiveComponent.SetCustomDepthStencilValue` (`self.Mesh`) 0)))

(fn `UpdateHealthBar`
  (bind _healthbar_w (`self.HealthBar_W`))
  (if (not (`self.Dead`))
    (bind _aswb_enemy_health (cast `/Game/UI/HUD/WB_EnemyHealth` (`WidgetComponent.GetWidget` (`self.HealthBar_W`))))
    (`ProgressBar.SetPercent` (`/Game/UI/HUD/WB_EnemyHealth.Healthbar` _aswb_enemy_health) (/ (`self.Health`) 100.0))
    (`SceneComponent.K2_SetWorldRotation` _healthbar_w (`KismetMathLibrary.FindLookAtRotation` (`SceneComponent.K2_GetComponentLocation` _healthbar_w) (`SceneComponent.K2_GetComponentLocation` (`Actor.RootComponent` (`GameplayStatics.GetPlayerCameraManager` 0)))) false false)))

(fn `UserConstructionScript`)