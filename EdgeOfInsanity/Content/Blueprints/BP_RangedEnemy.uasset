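; BP_RangedEnemy is a turret-like enemy that shoots projectiles at the player within range.
; Tick turns its head toward the player with clamped pitch and uses a Delay to pace projectile spawns, each launched by an impulse.
; It also updates a camera-facing health bar.
; TakeDamage lowers health, then destroys the actor without branching on death, changes the player's blood and clears any lock-on to it.
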(event `self.ReceiveTick`
  (params (DeltaSeconds :type "Float (single-precision)"))
  (bind (_returnvalue_roll _returnvalue_pitch _returnvalue_yaw) (`KismetMathLibrary.BreakRotator` (`KismetMathLibrary.FindLookAtRotation` (`self.K2_GetActorLocation`) (`self.K2_GetActorLocation` (`GameplayStatics.GetPlayerCharacter` 0)))))
  ;[1 1 1] detect and spawn
  (`self.UpdateHealthbar`)
  (if (< (`KismetMathLibrary.Vector_Distance` (`self.K2_GetActorLocation`) (`self.K2_GetActorLocation` (`GameplayStatics.GetPlayerCharacter` 0))) 2000.0)
    (`SceneComponent.K2_SetWorldRotation` (`self.Head`) (`KismetMathLibrary.MakeRotator` _returnvalue_roll (`KismetMathLibrary.ClampAngle` _returnvalue_pitch 0.0 90.0) _returnvalue_yaw) false false)
    (`KismetSystemLibrary.Delay` 0.4)
    (bind _returnvalue (`|SpawnActorFromClass` "/Game/Blueprints/BP_RangedEnemyProjectile.BP_RangedEnemyProjectile_C" (`SceneComponent.K2_GetComponentToWorld` (`self.ProjectileSpawnPoint`)) "Undefined" "MultiplyWithRoot" null null))
    (`PrimitiveComponent.AddImpulse` (`/Game/Blueprints/BP_RangedEnemyProjectile.Sphere` _returnvalue) (* (`SceneComponent.GetForwardVector` (`/Game/Blueprints/BP_RangedEnemyProjectile.Sphere` _returnvalue)) 300.0) "None" false)))

(event `Take Damage`
  (params (damage :type "Float (double-precision)") (BloodOffset :type "Float (double-precision)" :default 10.0))
  ;[1 1 1] Take Damage
  (bind _output_get (set `self.Health` (- (`self.Health`) damage)))
  (set `self.Dead` (<= _output_get 0.0))
  (`GameplayStatics.PlaySound2D` "/Game/StarterContent/Audio/Explosion01.Explosion01" 0.25 1.0 0.0 null null)
  (`self.K2_DestroyActor`)
  (bind _asbp_third_person_character (cast `/Game/Blueprints/BP_ThirdPersonCharacter` (`GameplayStatics.GetPlayerPawn` 0)))
  (`/Game/Blueprints/BP_ThirdPersonCharacter.ChangeBlood` _asbp_third_person_character BloodOffset)
  (`self.ClearLockOn`))

(fn `ClearLockOn`
  (bind _asbp_third_person_character (cast `/Game/Blueprints/BP_ThirdPersonCharacter` (`GameplayStatics.GetPlayerPawn` 0)))
  (if (== (`/Game/Blueprints/BP_ThirdPersonCharacter.LockOnTarget` _asbp_third_person_character) self)
    (set `/Game/Blueprints/BP_ThirdPersonCharacter.LockOnTarget` null _asbp_third_person_character)))

(fn `UpdateHealthbar`
  (bind _healthbar_w (`self.HealthBar_W`))
  (if (not (`self.Dead`))
    (bind _aswb_enemy_health (cast `/Game/UI/HUD/WB_EnemyHealth` (`WidgetComponent.GetWidget` (`self.HealthBar_W`))))
    (`ProgressBar.SetPercent` (`/Game/UI/HUD/WB_EnemyHealth.Healthbar` _aswb_enemy_health) (/ (`self.Health`) 100.0))
    (`SceneComponent.K2_SetWorldRotation` _healthbar_w (`KismetMathLibrary.FindLookAtRotation` (`SceneComponent.K2_GetComponentLocation` _healthbar_w) (`SceneComponent.K2_GetComponentLocation` (`Actor.RootComponent` (`GameplayStatics.GetPlayerCameraManager` 0)))) false false)))

(fn `UserConstructionScript`)