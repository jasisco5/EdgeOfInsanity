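; BP_Fireball is a homing projectile that plays a sound on spawn and self-destructs after a short lifetime or on hit.
; Its Detection overlap locks onto the first living melee or ranged enemy, ignoring BP_EnemyAI's PlayerDetection component.
; Tick eases rotation toward that target and moves forward by a fixed, frame-rate-dependent step.
; With a target locked, overlapping either enemy type calls TakeDamage and destroys the fireball, though ranged enemies receive zero damage.
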(event `self.ReceiveBeginPlay`
  (`GameplayStatics.PlaySound2D` "/Game/Audio/fireball.fireball" 1.0 1.0 0.0 null null)
  (`KismetSystemLibrary.Delay` 5.0)
  (`self.K2_DestroyActor`))

(event `self.ReceiveTick`
  (params (DeltaSeconds :type "Float (single-precision)"))
  (`/Engine/EditorBlueprintResources/StandardMacros.IsValid` (`self.HuntTarget`)
    (:`Is Valid`
      (`self.K2_SetActorRotation` (`KismetMathLibrary.RInterpTo` (`self.K2_GetActorRotation`) (`KismetMathLibrary.FindLookAtRotation` (`self.K2_GetActorLocation`) (`self.K2_GetActorLocation` (`self.HuntTarget`))) DeltaSeconds 3.0)))
    (:`Is Not Valid`
      _))
  (`SceneComponent.K2_AddWorldOffset` (`self.Scene`) (* (`self.GetActorForwardVector`) 15.0) false false))

(event `self.Fireball.OnComponentHit`
  (params (HitComponent :type "PrimitiveComponent Object Reference") (OtherActor :type "Actor Object Reference") (OtherComp :type "PrimitiveComponent Object Reference") (NormalImpulse :type "Vector Structure") (Hit :type "HitResult Structure (by ref)"))
  (`self.K2_DestroyActor`))

(event `self.Fireball.OnComponentBeginOverlap`
  (params (OverlappedComponent :type "PrimitiveComponent Object Reference") (OtherActor :type "Actor Object Reference") (OtherComp :type "PrimitiveComponent Object Reference") (OtherBodyIndex :type Integer) (bFromSweep :type Boolean) (SweepResult :type "HitResult Structure (by ref)"))
  (bind _asbp_enemy_ai (cast `/Game/Blueprints/BP_EnemyAI` OtherActor)
    (:`then`
      (`/Engine/EditorBlueprintResources/StandardMacros.IsValid` (`self.HuntTarget`)
        (:`Is Valid`
          (`/Game/Blueprints/BP_EnemyAI.TakeDamage` _asbp_enemy_ai false 100.0 5.0))))
    (:`CastFailed`
      (bind _asbp_ranged_enemy (cast `/Game/Blueprints/BP_RangedEnemy` OtherActor))
      (`/Engine/EditorBlueprintResources/StandardMacros.IsValid` (`self.HuntTarget`)
        (:`Is Valid`
          (`/Game/Blueprints/BP_RangedEnemy.Take Damage` _asbp_ranged_enemy 0.0 5.0)))))
  (`self.K2_DestroyActor`))

(event `self.Detection.OnComponentBeginOverlap`
  (params (OverlappedComponent :type "PrimitiveComponent Object Reference") (OtherActor :type "Actor Object Reference") (OtherComp :type "PrimitiveComponent Object Reference") (OtherBodyIndex :type Integer) (bFromSweep :type Boolean) (SweepResult :type "HitResult Structure (by ref)"))
  (bind _asbp_enemy_ai (cast `/Game/Blueprints/BP_EnemyAI` OtherActor)
    (:`then`
      (if (!= (`/Game/Blueprints/BP_EnemyAI.PlayerDetection` _asbp_enemy_ai) OtherComp)
        (`/Engine/EditorBlueprintResources/StandardMacros.IsValid` (`self.HuntTarget`)
          (:`Is Not Valid`
            (if (not (`/Game/Blueprints/BP_EnemyAI.Dead` _asbp_enemy_ai))
              (set `self.HuntTarget` _asbp_enemy_ai))))))
    (:`CastFailed`
      (bind _asbp_ranged_enemy (cast `/Game/Blueprints/BP_RangedEnemy` OtherActor))
      (`/Engine/EditorBlueprintResources/StandardMacros.IsValid` (`self.HuntTarget`)
        (:`Is Not Valid`
          (if (not (`/Game/Blueprints/BP_RangedEnemy.Dead` _asbp_ranged_enemy))
            (set `self.HuntTarget` _asbp_ranged_enemy)))))))

(fn `UserConstructionScript`)