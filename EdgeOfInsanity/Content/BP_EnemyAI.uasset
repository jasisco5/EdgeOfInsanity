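; BP_EnemyAI is a melee enemy that chases the player on sight and drains sanity with its punches.
; PawnSensing triggers an AI move, arrival plays the punch montage, and hand overlaps deal sanity damage only while attacking.
; TakeDamage permanently sets Frozen, disables capsule collision and ragdolls the mesh with an impulse away from the player.
; An older timed-freeze hit reaction using time dilation remains unconnected.
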(event `self.PawnSensing.OnSeePawn`
  (params (Pawn :type "Pawn Object Reference"))
  (`self.FollowPlayer`))

(event `FollowPlayer`
  (if (not (`self.frozen`))
    (`|AIMoveTo` self (0.0 0.0 0.0) (`GameplayStatics.GetPlayerCharacter` 0) 70.0
      (:`OnSuccess`
        (if (not (`self.isAttacking`))
          (set `self.isAttacking` true)
          (bind _returnvalue (`self.PlayAnimMontage` "/Game/Characters/Enemy/EnemyPunches_Montage.EnemyPunches_Montage"))
          (`KismetSystemLibrary.Delay` _returnvalue)
          (set `self.isAttacking` false))))))

(event `self.RightHand.OnComponentBeginOverlap`
  (params (OverlappedComponent :type "PrimitiveComponent Object Reference") (OtherActor :type "Actor Object Reference") (OtherComp :type "PrimitiveComponent Object Reference") (OtherBodyIndex :type Integer) (bFromSweep :type Boolean) (SweepResult :type "HitResult Structure (by ref)"))
  (bind _asbp_third_person_character (cast `/Game/ThirdPerson/Blueprints/BP_ThirdPersonCharacter` OtherActor))
  (if (and (not (`self.frozen`)) (`self.isAttacking`))
    (`/Game/ThirdPerson/Blueprints/BP_ThirdPersonCharacter.ChangeSanity` _asbp_third_person_character -5.0)))

(event `self.LeftHand.OnComponentBeginOverlap`
  (params (OverlappedComponent :type "PrimitiveComponent Object Reference") (OtherActor :type "Actor Object Reference") (OtherComp :type "PrimitiveComponent Object Reference") (OtherBodyIndex :type Integer) (bFromSweep :type Boolean) (SweepResult :type "HitResult Structure (by ref)"))
  (bind _asbp_third_person_character (cast `/Game/ThirdPerson/Blueprints/BP_ThirdPersonCharacter` OtherActor))
  (if (and (not (`self.frozen`)) (`self.isAttacking`))
    (`/Game/ThirdPerson/Blueprints/BP_ThirdPersonCharacter.ChangeSanity` _asbp_third_person_character -5.0)))

(event `TakeDamage`
  (set `self.frozen` true)
  (`PrimitiveComponent.SetCollisionEnabled` (`self.CapsuleComponent`) "NoCollision")
  (`PrimitiveComponent.SetSimulatePhysics` (`self.Mesh`) true)
  (`PrimitiveComponent.AddImpulse` (`self.Mesh`) (* (`KismetMathLibrary.GetDirectionUnitVector` (`self.K2_GetActorLocation` (`GameplayStatics.GetPlayerPawn` 0)) (`self.K2_GetActorLocation`)) 20000.0) "None" false))

(fn `UserConstructionScript`)